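; Speed trap that slows any BP_ThirdPersonCharacter inside its box by setting Ralentizar on overlap begin and clearing it on end.
; The server loops endlessly, switching the trap on and off at short random intervals through the Activo RepNotify variable.
; Encender and Apagar toggle the box's overlap events and the plane's dynamic material parameter, with OnRep_Activo mirroring the state on clients.
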(event OnComponentBeginOverlap(Box)
  (params (OverlappedComponent :type Primitive%20Component%20Object%20Reference) (OtherActor :type Actor%20Object%20Reference) (OtherComp :type Primitive%20Component%20Object%20Reference) (OtherBodyIndex :type Integer) (bFromSweep :type Boolean) (SweepResult :type Hit%20Result%20Structure%20%28by%20ref%29))
  (bind _asbp_third_person_character (Utilities|Casting|CastToBP_ThirdPersonCharacter OtherActor))
  (Default|SetRalentizar _asbp_third_person_character true))

(event OnComponentEndOverlap(Box)
  (params (OverlappedComponent :type Primitive%20Component%20Object%20Reference) (OtherActor :type Actor%20Object%20Reference) (OtherComp :type Primitive%20Component%20Object%20Reference) (OtherBodyIndex :type Integer))
  (bind _asbp_third_person_character (Utilities|Casting|CastToBP_ThirdPersonCharacter OtherActor))
  (Default|SetRalentizar _asbp_third_person_character false))

(event Custom|Encender
  (Rendering|Material|SetScalarParameterValue (Variables|Default|GetMaterial) "Encendido" 1.0 :!class /Script/Engine.MaterialInstanceDynamic)
  (Variables|/Script/Engine.PrimitiveComponent|SetbGenerateOverlapEvents (Variables|Default|GetBox) true))

(event Custom|Apagar
  (Rendering|Material|SetScalarParameterValue (Variables|Default|GetMaterial) "Encendido" 0.0 :!class /Script/Engine.MaterialInstanceDynamic)
  (Variables|/Script/Engine.PrimitiveComponent|SetbGenerateOverlapEvents (Variables|Default|GetBox) false))

(event EventBeginPlay
  ;[1 1 1] Establecer material dinámico
  (bind _returnvalue (Rendering|Material|CreateDynamicMaterialInstance (Variables|Default|GetPlane) 0 "/Game/Materials/MAT_TrampaVelocidad.MAT_TrampaVelocidad" "None" :!class /Script/Engine.PrimitiveComponent))
  (Variables|Default|SetMaterial _returnvalue)
  (Networking|SwitchHasAuthority
    (:Authority
      (Utilities|FlowControl|Delay (Math|Random|RandomFloatinRange 2.0 3.0) :!label _label)
      (Variables|Default|SetActivo true)
      (CallFunction|Encender)
      (Utilities|FlowControl|Delay (Math|Random|RandomFloatinRange 2.0 3.0))
      (CallFunction|Apagar)
      (Variables|Default|SetActivo false)
      (goto _label))))

(fn ConstructionScript)

(fn OnRepActivo
  (if (Variables|Default|GetActivo)
    (CallFunction|Encender)
    (else
      (CallFunction|Apagar))))
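; BP_BotonTriestadoMano is a tri-state button whose spotlight color shows its current state.
; Accionar fires the BotonPulsado dispatcher with the Personaje, then advances IndexColor through TriestadoColors, wrapping to the first, and recolors the light.
; The dispatcher fires before the index changes, so listeners run while the previous state is still set.
; The construction script sets the initial color, and an OnRep on IndexColor reapplies it on replication.
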(event Custom|UpdateIndexColor
  ;[1 1 1] si el index es > a los colores del botones vuelve al primer color, sino va al siguiente
  (if (>= (Variables|Default|GetindexColor) (- (Utilities|Array|Length (Variables|Default|Gettriestado_colors)) 1))
    (Variables|Default|SetindexColor 0) ; sumar +1 al index
    (else
      (Variables|Default|SetindexColor (+ (Variables|Default|GetindexColor) 1)) ; reiniciar index
    )))

(event EventBeginPlay)

(event Collision|EventActorBeginOverlap
  (params (OtherActor :type Actor%20Object%20Reference)))

(event EventTick
  (params (DeltaSeconds :type Float%20%28single-precision%29)))

(event EventAccionar
  (params (Personaje :type BP%20Third%20Person%20Character%20Object%20Reference))
  (Default|CallBotonPulsado Personaje)
  (CallFunction|UpdateIndexColor)
  (Rendering|Components|Light|SetLightColor (Variables|Default|GetSpotLight) (Utilities|Array|Get(acopy) (Variables|Default|Gettriestado_colors) (Variables|Default|GetindexColor)) true))

(fn ConstructionScript
  (Rendering|Components|Light|SetLightColor (Variables|Default|GetSpotLight) (Utilities|Array|Get(acopy) (Variables|Default|Gettriestado_colors) (Variables|Default|GetindexColor)) true))

(fn OnRepIndexColor
  (Rendering|Components|Light|SetLightColor (Variables|Default|GetSpotLight) (Utilities|Array|Get(acopy) (Variables|Default|Gettriestado_colors) (Variables|Default|GetindexColor)) true))
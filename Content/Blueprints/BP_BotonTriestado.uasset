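; BP_BotonTriestado is a button actor that cycles through colors each time something steps into its trigger box.
; Each begin overlap sets EstaActivo, advances IndexColor through TriestadoColors with wraparound, then shows the SpotLight in that color.
; When the last overlapping actor leaves the box, it clears EstaActivo and hides the light, keeping the index for the next activation.
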(event OnComponentBeginOverlap(Box)
  (params (OverlappedComponent :type Primitive%20Component%20Object%20Reference) (OtherActor :type Actor%20Object%20Reference) (OtherComp :type Primitive%20Component%20Object%20Reference) (OtherBodyIndex :type Integer) (bFromSweep :type Boolean) (SweepResult :type Hit%20Result%20Structure%20%28by%20ref%29))
  (Variables|Default|SetEstaActivo true)
  (CallFunction|UpdateIndexColor)
  (Rendering|Components|Light|SetLightColor (Variables|Default|GetSpotLight) (Utilities|Array|Get(acopy) (Variables|Default|Gettriestado_colors) (Variables|Default|GetindexColor)) true)
  (Rendering|SetVisibility (Variables|Default|GetSpotLight) true false))

(event OnComponentEndOverlap(Box)
  (params (OverlappedComponent :type Primitive%20Component%20Object%20Reference) (OtherActor :type Actor%20Object%20Reference) (OtherComp :type Primitive%20Component%20Object%20Reference) (OtherBodyIndex :type Integer))
  (if (== (Utilities|Array|Length (Collision|GetOverlappingActors (Variables|Default|GetBox) 0 :!class /Script/Engine.PrimitiveComponent)) 0)
    (Variables|Default|SetEstaActivo false)
    (Rendering|SetVisibility (Variables|Default|GetSpotLight) false false)))

(event Custom|UpdateIndexColor
  ;[1 1 1] si el index es > a los colores del botones vuelve al primer color, sino va al siguiente
  (if (>= (Variables|Default|GetindexColor) (- (Utilities|Array|Length (Variables|Default|Gettriestado_colors)) 1))
    (Variables|Default|SetindexColor 0) ; sumar +1 al index
    (else
      (Variables|Default|SetindexColor (+ (Variables|Default|GetindexColor) 1)) ; reiniciar index
    )))

(event EventBeginPlay)

(event Collision|EventActorBeginOverlap
  (params (OtherActor :type Actor%20Object%20Reference)))

(event EventTick
  (params (DeltaSeconds :type Float%20%28single-precision%29)))

(fn ConstructionScript)
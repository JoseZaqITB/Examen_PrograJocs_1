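; Automatic dispenser actor that spawns cubes of a configurable class at its own transform and replaces them when they disappear from the world.
; The construction script calls Generar, which spawns and records an actor, then re-calls itself after a delay while the count is below MaxCubes.
; Tick scans the tracked array, removes invalid entries, and triggers Generar again after the same GeneratorDelay.
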(event Custom|Generar
  (bind _currentcubes (Variables|Default|GetcurrentCubes))
  (bind _returnvalue (Game|SpawnActorfromClass (Variables|Default|GetClaseAGenerar) (Transformation|GetActorTransform) "Undefined" "MultiplyWithRoot" 0 0))
  ;[1 1 1] guarda el actor generado en el array currentCubes
  (Utilities|Array|Add _currentcubes _returnvalue)
  ;[1 1 1] si hay menos de 2 cubos generados, genera otro
  (if (< (Utilities|Array|Length _currentcubes) (Variables|Default|GetmaxCubes))
    (Utilities|FlowControl|Delay (Variables|Default|GetgeneratorDelay))
    (CallFunction|Generar)))

(event EventBeginPlay)

(event Collision|EventActorBeginOverlap
  (params (OtherActor :type Actor%20Object%20Reference)))

(event EventTick
  (params (DeltaSeconds :type Float%20%28single-precision%29))
  ;[1 1 1] si un cubo generado no esta en el mundo, se crea otro nuevo en 5seg
  (for (_array_element _array_index) (Variables|Default|GetcurrentCubes)
    (Utilities|IsValid _array_element
      (:Is%20Not%20Valid
        (Utilities|Array|RemoveIndex (Variables|Default|GetcurrentCubes) _array_index)
        (Utilities|FlowControl|Delay (Variables|Default|GetgeneratorDelay))
        (CallFunction|Generar)))))

(fn ConstructionScript
  (CallFunction|Generar))
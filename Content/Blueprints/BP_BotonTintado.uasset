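; BP_BotonTintado is a color-coded button that activates while a BP_ThirdPersonCharacter whose ColorPersonaje matches its ColorRequerido overlaps its Box.
; The construction script tints the cylinder with the required color through a dynamic material instance.
; Overlap events set EstaActivo and SpotLight visibility, with end overlap rechecking remaining actors for a match.
; EstaActivo's RepNotify mirrors the light state on replication.
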(event OnComponentBeginOverlap(Box)
  (params (OverlappedComponent :type Primitive%20Component%20Object%20Reference) (OtherActor :type Actor%20Object%20Reference) (OtherComp :type Primitive%20Component%20Object%20Reference) (OtherBodyIndex :type Integer) (bFromSweep :type Boolean) (SweepResult :type Hit%20Result%20Structure%20%28by%20ref%29))
  (bind _asbp_third_person_character (Utilities|Casting|CastToBP_ThirdPersonCharacter OtherActor))
  (if (Utilities|Enum|Equal(Enum) (Variables|/Game/ThirdPerson/Blueprints/BP_ThirdPersonCharacter.BP_ThirdPersonCharacter_C|GetColorPersonaje _asbp_third_person_character) (Variables|Default|GetColorRequerido))
    (Variables|Default|SetEstaActivo true)
    (Rendering|SetVisibility (Variables|Default|GetSpotLight) true false)))

(event OnComponentEndOverlap(Box)
  (params (OverlappedComponent :type Primitive%20Component%20Object%20Reference) (OtherActor :type Actor%20Object%20Reference) (OtherComp :type Primitive%20Component%20Object%20Reference) (OtherBodyIndex :type Integer))
  (Variables|Default|SetEstaActivo false)
  (Rendering|SetVisibility (Variables|Default|GetSpotLight) false false)
  (for _array_element (Collision|GetOverlappingActors (Variables|Default|GetBox) 0 :!class /Script/Engine.PrimitiveComponent)
    (bind _asbp_third_person_character (Utilities|Casting|CastToBP_ThirdPersonCharacter _array_element))
    (if (Utilities|Enum|Equal(Enum) (Variables|/Game/ThirdPerson/Blueprints/BP_ThirdPersonCharacter.BP_ThirdPersonCharacter_C|GetColorPersonaje _asbp_third_person_character) (Variables|Default|GetColorRequerido))
      (Variables|Default|SetEstaActivo true)
      (Rendering|SetVisibility (Variables|Default|GetSpotLight) true false))))

(fn ConstructionScript
  (bind _returnvalue (Rendering|Material|CreateDynamicMaterialInstance (Variables|Default|GetCylinder) 0 "/Engine/BasicShapes/BasicShapeMaterial.BasicShapeMaterial" "None" :!class /Script/Engine.PrimitiveComponent))
  (bind _output_get (Variables|Default|SetMaterial _returnvalue))
  (Rendering|Material|SetVectorParameterValue _output_get "Color" (CallFunction|GetColorPersonaje (Variables|Default|GetColorRequerido)) :!class /Script/Engine.MaterialInstanceDynamic))

(fn OnRepEstaActivo
  (if (Variables|Default|GetEstaActivo)
    (Rendering|SetVisibility (Variables|Default|GetSpotLight) true false)
    (else
      (Rendering|SetVisibility (Variables|Default|GetSpotLight) false false))))